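; Base weapon item Blueprint that turns its WeaponInfo type, rolls and item level into a name and core combat stats on BeginPlay.
; Looks up the weapon type's base stats in a data table, then derives attack speed from a quality roll and damage range from spread rolls scaled by item level.
; Subclass, optional prefix and optional suffix table rows supply name parts and roll-driven stat changes layered onto those stats.
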(event EventBeginPlay
  (bind _weaponinfo (Variables|Default|GetWeaponInfo))
  (bind (_type _maxdamagespreadroll _mindamagespreadroll _attackspeedroll _socketroll _itemlevel _subclass _subclassroll _hasprefix _prefix _prefixroll _hassuffix _suffix _suffixroll) (Utilities|Struct|BreakStructure_WeaponInfo _weaponinfo))
  (bind (_damagemodel _maxdamagespread _mindamagespread _maxspeed _minspeed) (Utilities|FindWeaponBaseStats _type)
    (:Finish
      (Variables|Default|SetCoreStats (Utilities|Struct|MakeStructre_CoreStats 0 0 0 0 0 0 0 (Utilities|FindAttackSpeed _maxspeed _minspeed _attackspeedroll) (Utilities|FindDamageRange _damagemodel _maxdamagespread _mindamagespread _maxdamagespreadroll _mindamagespreadroll _itemlevel) "(MinDamage_3_A5B3F499417FF31D6E649496EFFF76D1=0,MaxDamage_5_13990EF04C9B10BDBC6C9C8E2636DEEC=0)" "(MinDamage_3_A5B3F499417FF31D6E649496EFFF76D1=0,MaxDamage_5_13990EF04C9B10BDBC6C9C8E2636DEEC=0)" "(MinDamage_3_A5B3F499417FF31D6E649496EFFF76D1=0,MaxDamage_5_13990EF04C9B10BDBC6C9C8E2636DEEC=0)" "(MinDamage_3_A5B3F499417FF31D6E649496EFFF76D1=0,MaxDamage_5_13990EF04C9B10BDBC6C9C8E2636DEEC=0)" "(MinDamage_3_A5B3F499417FF31D6E649496EFFF76D1=0,MaxDamage_5_13990EF04C9B10BDBC6C9C8E2636DEEC=0)"))
      (Utilities|SetName
        (:Finish
          (Utilities|ApplySubClass _subclass _subclassroll
            (:Finish
              (if _hasprefix
                (Utilities|ApplyPrefix _prefix _prefixroll
                  (:Finish
                    _)))
              (if _hassuffix
                (Utilities|ApplySuffix _suffix _suffixroll)))))))))

(fn ConstructionScript
  (|CallParentFunction))